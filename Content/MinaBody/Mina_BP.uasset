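; Mina_BP is a Blueprint that handles the Pause Game input action to toggle the game's pause menu.
; On press it creates the PauseMenu widget if the stored reference is invalid, then branches on whether the game is paused.
; Pausing shows the menu with Game and UI input focused on it; unpausing removes it and restores game-only input.
; Both branches keep the mouse cursor hidden.
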(event Input|ActionEvents|InputActionPauseGame
  (params (Key :type Key%20Structure :default "None"))
  (bind _returnvalue (Game|GetPlayerController 0))
  ;[1 1 1] Pause and Unpause Game
  (:Pressed
    (Utilities|IsValid (Variables|Default|GetPause%20Menu%20Reference)
      (:Is%20Valid
        _)
      (:Is%20Not%20Valid
        (bind _returnvalue_2 (UserInterface|CreateWidget "/Game/MenusAndSettings/PauseMenu.PauseMenu_C"))
        (Variables|Default|SetPause%20Menu%20Reference _returnvalue_2)))
    (if (Game|IsGamePaused)
      (Widget|RemovefromParent (Variables|Default|GetPause%20Menu%20Reference))
      (Game|SetGamePaused false)
      (Variables|/Script/Engine.PlayerController|SetbShowMouseCursor _returnvalue false)
      (Input|SetInputModeGameOnly _returnvalue)
      (else
        (UserInterface|Viewport|AddtoViewport (Variables|Default|GetPause%20Menu%20Reference) 0)
        (Game|SetGamePaused true)
        (Variables|/Script/Engine.PlayerController|SetbShowMouseCursor _returnvalue false)
        (Input|SetInputModeGameandUI _returnvalue (Variables|Default|GetPause%20Menu%20Reference) "LockInFullscreen" false)))))

(fn ConstructionScript)