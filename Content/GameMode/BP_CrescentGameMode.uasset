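; BP_CrescentGameMode is a game mode Blueprint that respawns the player's Mina_BP character whenever it is destroyed.
; On BeginPlay it casts player character 0 to Mina_BP and binds to its OnDestroyed event.
; After a short delay, the handler spawns a new Mina_BP at SpawnTransform, has player controller 0 possess it, then calls Respawn to rebind for the next death.
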(event Custom|On%20Destroyed
  (params (DestroyedActor :type Actor%20Object%20Reference))
  ;[1 1 1] Respawn System
  (Utilities|FlowControl|Delay 2.0)
  (bind _returnvalue (Game|SpawnActorfromClass "/Game/MinaBody/Mina_BP.Mina_BP_C" (Variables|Default|GetSpawn%20Transform) "Undefined" 0 0))
  (Pawn|Possess (Game|GetPlayerController 0) _returnvalue)
  (CallFunction|Respawn))

(event Custom|Respawn
  ;[1 1 1] Respawn System
  (bind _asmina_bp (Utilities|Casting|CastToMina_BP (Game|GetPlayerCharacter 0)))
  (Game|BindEventtoOnDestroyed _asmina_bp (delegate Custom|On%20Destroyed)))

(event EventBeginPlay
  ;[1 1 1] Respawn System
  (bind _asmina_bp (Utilities|Casting|CastToMina_BP (Game|GetPlayerCharacter 0)))
  (Game|BindEventtoOnDestroyed _asmina_bp (delegate Custom|On%20Destroyed)))

(fn ConstructionScript)